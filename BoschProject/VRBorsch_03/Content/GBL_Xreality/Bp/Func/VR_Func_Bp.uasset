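; VR_Func_Bp is a shared helper library for VR popup UI, level transitions and small lookups.
; Popups are created through VR_SpawnerUI with the VRPopup_Bp class.
; A target level name is saved in a SaveLevel object under a fixed slot, with an existence check, while the open-next-level function always loads Lobby_Level rather than reading that save.
; Other helpers fetch level-info data table rows and test whether two tag sets share any element.
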(fn `Fc Tag Matching`
  (params (TagA :type "Array of Name") (TagB :type "Array of Name"))
  (returns (Success :type Boolean))
  (for _array_element TagA
    (if (`KismetArrayLibrary.Array_Contains` TagB _array_element)
      (return true)))
  (return false))

(fn `Fc_CheckSaveValid`
  (returns (isValid :type Boolean))
  (bind _returnvalue (`GameplayStatics.DoesSaveGameExist` (`self.Fc_DefaultSaveName` null)))
  (return _returnvalue))

(fn `Fc_DefaultSaveName`
  (returns (savName :type String))
  (return "boschsave"))

(fn `Fc_LevelInfomation`
  (params (Name :type "DataTableRowHandle Structure"))
  (returns (`Out Row` :type "/Game/BoschVR/Data/VRLevelStruct Structure"))
  (bind (_datatable _rowname) (break `DataTableRowHandle` Name))
  (bind _returnvalue (`|GetDataTableRow` _datatable _rowname)
    (:`then`
      (return _returnvalue))))

(fn `Fc_OpenToNextLevel`
  (`GameplayStatics.OpenLevel` null "Lobby_Level"))

(fn `Fc_PopupUiActor`
  (params (Params :type String))
  (`|CreateWidget` "/Game/GBL_Xreality/Bp/UI/Common/VR_SpawnerUI.VR_SpawnerUI_C" null "/Game/GBL_Xreality/Bp/Actors/VRPopup_Bp.VRPopup_Bp_C" Params))

(fn `Fc_SaveNextLevelName`
  (params (LevelName :type String))
  (bind _returnvalue (`GameplayStatics.CreateSaveGameObject` "/Game/BoschVR/Data/SaveLevel.SaveLevel_C"))
  (set `/Game/BoschVR/Data/SaveLevel.ToLevel` LevelName _returnvalue)
  (`GameplayStatics.SaveGameToSlot` _returnvalue (`self.Fc_DefaultSaveName` null)))