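; VR popup actor that shows a title and text lines in a widget and closes when touched.
; On BeginPlay it sets the widget's input action priority, sends it the info through an interface message, and binds to the touch dispatcher.
; A touch sends a "touchDamage" message with its BID to the attach parent actor, then closes the popup, spawning a close effect and destroying the actor.
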(event `self.IBP_CloseUI`
  (`GameplayStatics.SpawnEmitterAtLocation` (`self.CloseEffect`) (`self.K2_GetActorLocation`))
  (`self.K2_DestroyActor`))

(event `OnTouch`
  (message `/Game/GBL_Xreality/Bp/Interfaces/IBP_VRTouch.IBP_VRTouching` (`self.GetAttachParentActor`) (`self.BID`) self "touchDamage")
  (`self.IBP_CloseUI`))

(event `self.ReceiveBeginPlay`
  (bind _returnvalue (`WidgetComponent.GetUserWidgetObject` (`self.Popup`)))
  (`UserWidget.SetInputActionPriority` _returnvalue 1)
  (message `/Game/GBL_Xreality/Bp/Interfaces/IBP_VRUI.IBP_VRInfo` _returnvalue (`self.Title`) (`self.Lines`) self)
  (`parent.ReceiveBeginPlay`)
  (add `self.DOnTouch` (delegate `OnTouch`)))

(fn `UserConstructionScript`)