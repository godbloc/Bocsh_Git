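; VR slot actor that holds a grabbable actor dropped inside its Box.
; Overlapping an empty slot reveals the Box and, for actors with a GrabComponent, binds their drop event to snap-attach them with physics off.
; Insertion and release fire dispatchers and swap the particle effect; release occurs on end overlap if the item's parent actor is not the slot.
; Interface functions are mostly stubs, apart from returning the first tag.
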(event `KeepInSlot`
  (bind _returnvalue (`self.GetComponentByClass` (stale `self.Box.OnComponentBeginOverlap` OtherActor) "/Game/VRTemplate/Blueprints/GrabComponent.GrabComponent_C"))
  (`/Game/VRTemplate/Blueprints/GrabComponent.SetPrimitiveCompPhysics` _returnvalue false)
  (`SceneComponent.K2_AttachToComponent` (`SceneComponent.GetAttachParent` _returnvalue) (`self.Box`) "None" "SnapToTarget" "SnapToTarget" "KeepWorld" true)
  (`SceneComponent.SetHiddenInGame` (`self.Box`) true false)
  (remove `/Game/VRTemplate/Blueprints/GrabComponent.OnDropped` _returnvalue (delegate `KeepInSlot`))
  (set `self.AInslot` (stale `self.Box.OnComponentBeginOverlap` OtherActor))
  (`self.DOnInsertActor` (stale `self.Box.OnComponentBeginOverlap` OtherActor))
  (`ParticleSystemComponent.SetTemplate` (`self.ParticleSystem`) (`self.InsertedFx`)))

(event `self.Box.OnComponentBeginOverlap`
  (params (OverlappedComponent :type "PrimitiveComponent Object Reference") (OtherActor :type "Actor Object Reference") (OtherComp :type "PrimitiveComponent Object Reference") (OtherBodyIndex :type Integer) (bFromSweep :type Boolean) (SweepResult :type "HitResult Structure (by ref)"))
  (bind _returnvalue (`self.GetComponentByClass` OtherActor "/Game/VRTemplate/Blueprints/GrabComponent.GrabComponent_C"))
  (`/Engine/EditorBlueprintResources/StandardMacros.IsValid` (`self.AInslot`)
    (:`Is Not Valid`
      (`/Engine/EditorBlueprintResources/StandardMacros.IsValid` _returnvalue
        (:`Is Valid`
          (add `/Game/VRTemplate/Blueprints/GrabComponent.OnDropped` _returnvalue (delegate `KeepInSlot`))
          (`SceneComponent.SetHiddenInGame` (`self.Box`) false false))
        (:`Is Not Valid`
          (`SceneComponent.SetHiddenInGame` (`self.Box`) false false))))))

(event `self.Box.OnComponentEndOverlap`
  (params (OverlappedComponent :type "PrimitiveComponent Object Reference") (OtherActor :type "Actor Object Reference") (OtherComp :type "PrimitiveComponent Object Reference") (OtherBodyIndex :type Integer))
  (bind _ainslot (`self.AInslot`))
  (`/Engine/EditorBlueprintResources/StandardMacros.IsValid` _ainslot
    (:`Is Valid`
      (if (and (== _ainslot OtherActor) (== (== (`self.GetParentActor` _ainslot) self) false))
        (`/Engine/EditorBlueprintResources/StandardMacros.IsValid` (`self.GetComponentByClass` OtherActor "/Game/VRTemplate/Blueprints/GrabComponent.GrabComponent_C")
          (:`Is Valid`
            (`SceneComponent.SetHiddenInGame` (`self.Box`) true false)
            (`self.DOnReleaseActor` _ainslot)
            (set `self.AInslot` null)
            (`ParticleSystemComponent.SetTemplate` (`self.ParticleSystem`) "/Game/InfinityBladeEffects/Effects/FX_Ambient/UI_MainMenu/P_Select_indicator1.P_Select_indicator1")))))))

(fn `ibp_CheckTagFilter`
  (params (TagName :type "Actor Object Reference"))
  (returns (Success :type Boolean))
  (return false))

(fn `Ibp_CurrentLevelSave`
  (returns (LevelName :type String))
  (return ""))

(fn `Ibp_VrCleanState`
  (returns (CompleteState :type Boolean) (Params :type String) (BID :type Integer))
  (return false "" 0))

(fn `ibp_VrTagName`
  (returns (TagName :type Name))
  (return (`|GetArrayItem` (`self.Tags`))))

(fn `RefActor`
  (returns (valid :type Boolean) (ReturnValue :type "Actor Object Reference"))
  (bind _returnvalue (`self.GetAttachParentActor`))
  (return (`KismetSystemLibrary.IsValid` _returnvalue) _returnvalue))

(fn `UserConstructionScript`
  (`parent.UserConstructionScript`))