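; SlotMachine_Bp is a slot actor that reports object insertion and removal to the actor it is attached to.
; On BeginPlay it binds handlers to its insert and release dispatchers.
; Each handler forwards the object, the slot itself, Params and BID to the attach parent through interface messages, leaving the response to that parent.
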(event `OnInsertA` :!signature `self.DOnInsertActor`
  (params (A :type "Actor Object Reference"))
  (message `/Game/GBL_Xreality/Bp/Interfaces/IBP_VirtualMachine.Ibp_InsertObjectToSlot` (`self.GetAttachParentActor`) A self (`self.Params`) (`self.BID`)))

(event `self.ReceiveBeginPlay`
  (`parent.ReceiveBeginPlay`)
  (add `self.DOnInsertActor` (delegate `OnInsertA`))
  (add `self.DOnReleaseActor` (delegate `OnGetOut`)))

(event `OnGetOut` :!signature `self.DOnReleaseActor`
  (params (A :type "Actor Object Reference"))
  (message `/Game/GBL_Xreality/Bp/Interfaces/IBP_VirtualMachine.Ibp_TakeOffObjectFromSlot` (`self.GetAttachParentActor`) A self (`self.BID`) (`self.Params`)))

(fn `UserConstructionScript`
  (`parent.UserConstructionScript`))