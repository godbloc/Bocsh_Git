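; SlotHolder is an interactable slot actor that accepts an inserted object and completes a machine task when that object reports a completed clean state.
; Its start interface event shows a warm particle effect.
; A valid insert notifies MachineFuncComp, then after a zero-length delay expires the object shortly and switches to the finish effect.
; Socket queries return the UIPlace transforms, machine state always reports unpowered and not ready, and removal does nothing.
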(event `/Game/GBL_Xreality/Bp/Interfaces/IBP_VirtualMachine.Ibp_Start`
  (`ParticleSystemComponent.SetTemplate` (`self.ParticleSystem`) (`self.Warm`)))

(event `/Game/GBL_Xreality/Bp/Interfaces/IBP_VirtualMachine.Ibp_TakeOffObjectFromSlot`
  (params (Ref :type "Actor Object Reference") (Slot :type "Actor Object Reference") (BID :type Integer) (Params :type String)))

(event `/Game/GBL_Xreality/Bp/Interfaces/IBP_VirtualMachine.Ibp_InsertObjectToSlot`
  (params (ref :type "Actor Object Reference") (fromSlot :type "Actor Object Reference") (params :type String) (BID :type Integer))
  (bind _completestate (message `/Game/GBL_Xreality/Bp/Interfaces/IBP_XVR.Ibp_VrCleanState` ref))
  (if _completestate
    (`/Game/BoschVR/BP/Comp/MachineFunc_Comp.CompleteFunctionTask` (`self.MachineFunc_Comp`))
    (`KismetSystemLibrary.Delay` 0.0)
    (`self.SetLifeSpan` ref 1.0)
    (`ParticleSystemComponent.SetTemplate` (`self.ParticleSystem`) (`self.finishFx`))))

(fn `Ibp_GetVirtualSocketTransform`
  (params (SocketName :type String) (Slot :type Integer))
  (returns (WorldTrans :type "Transform Structure") (LocalTrans :type "Transform Structure"))
  (bind _uiplace (`self.UIPlace`))
  (return (`SceneComponent.K2_GetComponentToWorld` _uiplace) (`SceneComponent.GetRelativeTransform` _uiplace)))

(fn `ibp_MachineState`
  (returns (powered :type Boolean) (Ready :type Boolean))
  (return false false))

(fn `UserConstructionScript`)