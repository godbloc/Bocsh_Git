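; Configurable machine actor that takes its skeletal mesh and animation blueprint from a data table row.
; The construction script calls SetupMachine, which looks up the row selected by the MachineType row handle, adds a skeletal mesh component if none exists, then applies the row's mesh and anim class.
; The TypeID input is unused, and BeginPlay, overlap and Tick are disabled stubs.
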(event `SetupMachine`
  (params (TypeID :type Integer))
  (bind _returnvalue (`self.GetComponentByClass` "/Script/Engine.SkeletalMeshComponent"))
  (bind (_datatable _rowname) (break `DataTableRowHandle` (`self.MachineType`)))
  (bind _returnvalue_2 (`|GetDataTableRow` _datatable _rowname)
    (:`then`
      (`/Engine/EditorBlueprintResources/StandardMacros.IsValid` _returnvalue
        (:`Is Valid`
          _)
        (:`Is Not Valid`
          (`AddComponent|NODE_AddSkeletalMeshComponent-0`)))
      (bind (_available _displayname _srank _typecode _mesh _actorclass _state _iconstate _animbp) (break `/Game/BoschVR/Data/VrMachinePropertiesStruct` _returnvalue_2))
      (`SkinnedMeshComponent.SetSkinnedAssetAndUpdate` _returnvalue _mesh true)
      (`SkeletalMeshComponent.SetAnimInstanceClass` _returnvalue _animbp))))

(fn `UserConstructionScript`
  (`parent.UserConstructionScript`)
  (`self.SetupMachine` 0))