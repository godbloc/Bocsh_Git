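; LeverTransien_Bp is a touchable level transition actor that represents one level, looked up by NameInfo.
; On touch it starts the transition through CompLevelTransient, spawns a "Level Loading" VR popup with the level's display name, and calls DOnActiveTransient.
; Its construction script always sets the 3D rank text.
; A self-resetting HasUpdate flag refreshes the level name and puts the level image on a dynamic material.
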(event `self.OnTouch`
  (bind _out_row (`/Game/GBL_Xreality/Bp/Func/VR_Func_Bp.Fc_LevelInfomation` (`self.NameInfo`)))
  (bind (_available _levelname _image _displayname) (break `/Game/BoschVR/Data/VRLevelStruct` _out_row))
  (`/Game/BoschVR/BP/Comp/Comp_LevelTransient.ActiveLevelTrans` (`self.Comp_LevelTransient`) _levelname)
  (`|SpawnActorFromClass` "/Game/GBL_Xreality/Bp/Actors/VRPopup_Bp.VRPopup_Bp_C" (`self.GetTransform`) "Undefined" "OverrideRootScale" null "Level Loading" _displayname "/Game/InfinityBladeEffects/Effects/FX_Treasure/Loot/P_KeyPickup_01.P_KeyPickup_01" null)
  (`self.DOnActiveTransient`))

(fn `UserConstructionScript`
  (bind _staticmesh (`self.StaticMesh`))
  (bind _mainmatindex (`self.MainMatIndex`))
  (bind _out_row (`/Game/GBL_Xreality/Bp/Func/VR_Func_Bp.Fc_LevelInfomation` (`self.NameInfo`)))
  (if (`self.hasUpdate`)
    (set `self.hasUpdate` false)
    (bind (_available _levelname _image _displayname _desc _rankname) (break `/Game/BoschVR/Data/VRLevelStruct` _out_row))
    (bind _output_get (set `self.Level Name` _levelname))
    (set `/Game/BoschVR/BP/Comp/Comp_LevelTransient.Level Name` _output_get (`self.Comp_LevelTransient`))
    (`|ExecutionSequence`
      (:`then_0`
        (bind _returnvalue (`PrimitiveComponent.CreateDynamicMaterialInstance` _staticmesh _mainmatindex (`PrimitiveComponent.GetMaterial` _staticmesh _mainmatindex) "None"))
        (`PrimitiveComponent.SetMaterial` _staticmesh _mainmatindex _returnvalue)
        (`MaterialInstanceDynamic.SetTextureParameterValue` _returnvalue "MainTex" _image))
      (:`then_1`
        (`TextRenderComponent.K2_SetText` (`self.3dName`) (`KismetTextLibrary.Conv_StringToText` _rankname) :!label _label)))
    (else
      (goto _label))))