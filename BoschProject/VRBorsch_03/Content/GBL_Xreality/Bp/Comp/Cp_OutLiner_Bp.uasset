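; Actor component that builds an outline object for its owner from a duplicate mesh with a self-illumination material.
; GetMeshTypeName resolves the mesh type, and MakeOutlinerObject handles only the Static case.
; That case adds a static mesh component tagged "outline", with a dynamic material on slot 0 whose "scale" parameter takes OutlineSize.
; The event graph runs nothing, so both functions require external calls.
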(fn `GetMeshTypeName`
  (set `self.MeshTypeName` (`|GetArrayItem` (`self.MeshTypeList`) (`self.MeshType`))))

(fn `MakeOutlinerObject`
  (params (NewMesh :type "StaticMesh Object Reference"))
  (switch `name` (`self.MeshTypeName`)
    (:`static`
      (bind _returnvalue (`|AddComponentByClass` (`self.GetOwner`) "/Script/Engine.StaticMeshComponent" false (`KismetMathLibrary.MakeTransform` (0.0 0.0 0.0))))
      (`StaticMeshComponent.SetStaticMesh` _returnvalue NewMesh)
      (bind _returnvalue_2 (`KismetMaterialLibrary.CreateDynamicMaterialInstance` "/Game/VRTemplate/Materials/Ma_SelfIlume_Inst.Ma_SelfIlume_Inst"))
      (`MaterialInstanceDynamic.SetScalarParameterValue` _returnvalue_2 "scale" (`self.OutlineSize`))
      (`PrimitiveComponent.SetMaterial` _returnvalue 0 _returnvalue_2)
      (set `ActorComponent.ComponentTags` (`|MakeArray` "outline" :!type "Name") _returnvalue))))