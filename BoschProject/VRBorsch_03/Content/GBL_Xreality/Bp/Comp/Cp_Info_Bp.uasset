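; Scene component that shows a floating info panel (title and text lines) on its owning actor in the XR project.
; After a one-second delay at BeginPlay, it finds a child widget component or creates and attaches one.
; Helper events build the text, and UpdateInfo sends it to the widget through an IBPVRInfoMessage call.
; Every tick it rotates to face the player camera.
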(event `MakeInFo`
  (params (Title :type String) (Lines :type String))
  (set `self.Title` Title)
  (set `self.Lines` Lines)
  (`self.UpdateInfo`))

(event `ClearLines`
  (set `self.Lines` ""))

(event `MakeLines`
  (params (Lines :type "Array of String"))
  (for _array_element Lines
    (set `self.Lines` (`KismetStringLibrary.Concat_StrStr` (`self.Lines`) " \n" _array_element))))

(event `MakeLineInfo`
  (params (ShortDesc :type String) (Time :type String) (State :type String))
  (set `self.Lines` (`KismetStringLibrary.Concat_StrStr` (`self.Lines`) ShortDesc " \n" Time " \n" State)))

(event `Initializing`
  (bind _returnvalue (`|AddComponentByClass` :`self` (`self.GetOwner`) :`Class` "/Script/UMG.WidgetComponent" :`bManualAttachment` true))
  (bind _returnvalue_2 (`|CreateWidget` (`self.Class`)))
  (`WidgetComponent.SetWidget` _returnvalue _returnvalue_2)
  (set `self.RefUi` _returnvalue)
  (`self.K2_AttachToComponent` _returnvalue self "None" "SnapToTarget" "SnapToTarget" "SnapToTarget" true)
  (set `self.UIObject` (`WidgetComponent.GetUserWidgetObject` _returnvalue)))

(event `UIRefCheck`
  (bind _refui (`self.RefUi`))
  (if (> (`self.GetNumChildrenComponents`) 0)
    (for _array_element (`self.GetChildrenComponents` false)
      (bind _aswidget_component (cast `WidgetComponent` _array_element))
      (set `self.RefUi` _aswidget_component))
    (`/Engine/EditorBlueprintResources/StandardMacros.IsValid` _refui
      (:`Is Valid`
        (bind _aswidget_component_2 (cast `WidgetComponent` _refui))
        (set `self.UIObject` (`WidgetComponent.GetUserWidgetObject` _aswidget_component_2)))
      (:`Is Not Valid`
        (`self.Initializing` :!label _label)))
    (else
      (goto _label))))

(event `self.ReceiveBeginPlay`
  (`KismetSystemLibrary.Delay` 1.0)
  (`self.UIRefCheck`)
  (`self.UpdateInfo`))

(event `UpdateInfo`
  (message `/Game/GBL_Xreality/Bp/Interfaces/IBP_VRUI.IBP_VRInfo` (`self.UIObject`) (`self.Title`) (`self.Lines`) (`self.GetOwner` self)))

(event `self.ReceiveTick`
  (params (DeltaSeconds :type "Float (single-precision)"))
  (`self.TrackToEye`))

(fn `TrackToEye`
  (`self.K2_SetWorldRotation` (`KismetMathLibrary.FindLookAtRotation` (`self.K2_GetComponentLocation`) (`PlayerCameraManager.GetCameraLocation` (`PlayerController.PlayerCameraManager` (`GameplayStatics.GetPlayerController` 0))))))

(fn `TrimTextLine`
  (params (CapChar :type Integer) (Text :type String))
  (returns (NewParam :type String))
  (return (`KismetMathLibrary.SelectString` (`KismetStringLibrary.GetSubstring` Text 0 CapChar) Text (> (`KismetStringLibrary.Len` Text) CapChar))))