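; Washing machine actor for VR whose open state (likely the door) toggles on each VR touch event.
; OpenMt and CloseMt set the state flag and play or reverse the SmoothOpenAuto timeline, which sends the open amount to BodyMesh's anim instance through an interface message.
; An external open message plays the full timeline when the amount is exactly one, and otherwise passes the amount straight to the anim instance.
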(event `/Game/GBL_Xreality/Bp/Interfaces/IBP_VRTouch.IBP_VRTouching`
  (params (BID :type Integer) (Sender :type "Actor Object Reference") (Params :type String))
  (if (`self.MtState`)
    (`self.CloseMt`)
    (else
      (`self.OpenMt`))))

(event `/Game/GBL_Xreality/Bp/Interfaces/IBP_VirtualMachine.Ibp_OpenMt`
  (params (OpenAmouth :type "Float (double-precision)") (FromSender :type "Actor Object Reference"))
  (if (== OpenAmouth 1.0)
    (`self.OpenMt`)
    (else
      (message `/Game/GBL_Xreality/Bp/Interfaces/IBP_VirtualMachine.Ibp_OpenMt` (`SkeletalMeshComponent.GetAnimInstance` (`self.BodyMesh`)) OpenAmouth self))))

(event `OpenMt`
  (set `self.MtState` true)
  (bind (_direction _openamouth) (`Timeline|SmoothOpenAuto` :!via `PlayFromStart` :!label _label)
    (:`Update`
      (message `/Game/GBL_Xreality/Bp/Interfaces/IBP_VirtualMachine.Ibp_OpenMt` (`SkeletalMeshComponent.GetAnimInstance` (`self.BodyMesh`)) _openamouth self))))

(event `CloseMt`
  (set `self.MtState` false)
  (goto _label :!via `ReverseFromEnd`))

(fn `UserConstructionScript`)