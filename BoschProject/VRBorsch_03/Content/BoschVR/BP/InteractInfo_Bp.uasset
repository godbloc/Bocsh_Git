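; InteractInfo_Bp is a touch-interactive info actor that shows or hides a popup widget in the game.
; InitUI creates the widget from UiClass and sets it on the scaled Popup component, at construction or when the control-UI interface call supplies a new class.
; OnTouch flips ShowUi to toggle visibility.
; Interface functions expose the Popup's transform as a virtual socket and always report an unpowered, not-ready machine state.
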(event `self.OnTouch`
  (bind _returnvalue (not (`self.ShowUi`)))
  (`parent.OnTouch`)
  (set `self.ShowUi` _returnvalue)
  (`SceneComponent.SetHiddenInGame` (`self.Popup`) _returnvalue false))

(event `/Game/GBL_Xreality/Bp/Interfaces/IBP_VirtualMachine.ibp_InitControlUI`
  (params (UIClass :type "UserWidget Class Reference") (Sender :type "Actor Object Reference"))
  (set `self.Ui Class` UIClass)
  (`self.InitUI`))

(event `InitUI`
  (bind _popup (`self.Popup`))
  (bind _returnvalue (`|CreateWidget` (`self.Ui Class`)))
  (`WidgetComponent.SetWidget` _popup _returnvalue)
  (`SceneComponent.SetWorldScale3D` _popup (`KismetMathLibrary.Conv_DoubleToVector` (`self.ActualScale`))))

(fn `Ibp_GetVirtualSocketTransform`
  (params (SocketName :type String) (Slot :type Integer))
  (returns (WorldTrans :type "Transform Structure") (LocalTrans :type "Transform Structure"))
  (bind _returnvalue (`SceneComponent.K2_GetComponentToWorld` (`self.Popup`)))
  (return _returnvalue (`KismetMathLibrary.MakeTransform` (.location _returnvalue) (.rotation _returnvalue))))

(fn `ibp_MachineState`
  (returns (powered :type Boolean) (Ready :type Boolean))
  (return false false))

(fn `UserConstructionScript`
  (`parent.UserConstructionScript`)
  (`self.InitUI`))