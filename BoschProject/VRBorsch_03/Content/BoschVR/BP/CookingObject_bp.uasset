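; VR washable object, labeled as clothing despite its CookingObject name, that tracks clean/dirty and dry/wet states and reports complete when both clean and dry.
; Interface alpha events set DryState or invert washing progress into a dirt value driving a dynamic material and CleanState.
; RepNotifies refresh its Vietnamese info label.
; The construction script applies the filter tag, creates the material and picks the state effect from CleanState.
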(event `/Game/GBL_Xreality/Bp/Interfaces/IBP_XVR.Ibp_VRChangeStateAlpha`
  (params (NewState :type "Float (double-precision)") (Sender :type "Actor Object Reference") (Params :type String) (BID :type Integer))
  (switch `string` Params
    (:`Default`
      (bind _output_get (set `self.CurrentState` (- 1.0 (`KismetMathLibrary.FClamp` NewState)) :!label _label))
      (`self.ApplyNewState` _output_get))
    (:`washing`
      (goto _label))
    (:`dry`
      (set `self.DryState` (> NewState 0.0)))))

(event `ApplyNewState`
  (params (dirtAlpha :type "Float (single-precision)"))
  (`MaterialInstanceDynamic.SetScalarParameterValue` (`self.DynMap`) "state" dirtAlpha)
  (set `self.CleanState` (<= dirtAlpha 0.5)))

(event `self.UpdateObjectInfo`
  (`/Game/GBL_Xreality/Bp/Comp/Cp_Info_Bp.MakeInFo` (`self.ObjectInfoMation`) "Quần áo" (`self.infostate`)))

(event `self.ReceiveBeginPlay`
  (`self.UpdateObjectInfo`))

(fn `ibp_CheckTagFilter`
  (params (TagName :type "Actor Object Reference"))
  (returns (Success :type Boolean))
  (return false))

(fn `Ibp_CurrentLevelSave`
  (returns (LevelName :type String))
  (return ""))

(fn `Ibp_VrCleanState`
  (returns (CompleteState :type Boolean) (Params :type String) (BID :type Integer))
  (return (and (`self.CleanState`) (`self.DryState`)) "clean" 0))

(fn `ibp_VrTagName`
  (returns (TagName :type Name))
  (return (`self.ClassFilter`)))

(fn `infostate`
  (returns (ReturnValue :type String))
  (return (`KismetStringLibrary.Concat_StrStr` (`KismetMathLibrary.SelectString` "Sạch" "Bẩn" (`self.CleanState`)) " \n" (`KismetMathLibrary.SelectString` "Khô" "Ướt" (`self.DryState`)))))

(fn `OnRep_CleanState`
  (`self.UpdateObjectInfo`))

(fn `OnRep_DryState`
  (`self.UpdateObjectInfo`))

(fn `UserConstructionScript`
  (bind _staticmesh (`self.StaticMesh`))
  (bind _statefx (`self.StateFx`))
  (bind _nextstatematerial (`self.NextStateMaterial`))
  (set `self.Tags` (`|MakeArray` (`self.ClassFilter`)))
  (`parent.UserConstructionScript`)
  (bind _returnvalue (`KismetMaterialLibrary.CreateDynamicMaterialInstance` (select `bool` (`KismetSystemLibrary.IsValid` _nextstatematerial) :`false` (`PrimitiveComponent.GetMaterial` _staticmesh 0) :`true` _nextstatematerial :!type "MaterialInterface Object Reference")))
  (bind _output_get (set `self.DynMap` _returnvalue))
  (`PrimitiveComponent.SetMaterial` _staticmesh 0 _output_get)
  (`self.ApplyNewState` (`self.CurrentState`))
  (if (`self.CleanState`)
    (`ParticleSystemComponent.SetTemplate` _statefx (`self.TrueFx`))
    (else
      (`ParticleSystemComponent.SetTemplate` _statefx (`self.falseFx`)))))