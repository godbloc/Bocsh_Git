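; InteractBtn_Bp is a touchable interaction button for the BoschVR game, built as a child Blueprint that reacts to VR touch.
; The IBPVRTouching interface event fires the DOnTouch dispatcher, which is bound to OnTouch on BeginPlay.
; OnTouch forwards the touch to the attach parent actor through the same interface, passing its BID, itself and a "touchDamage" parameter, then spawns an impact particle at its location.
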(event `/Game/GBL_Xreality/Bp/Interfaces/IBP_VRTouch.IBP_VRTouching`
  (params (BID :type Integer) (Sender :type "Actor Object Reference") (Params :type String))
  (`self.DOnTouch`))

(event `OnTouch`
  (message `/Game/GBL_Xreality/Bp/Interfaces/IBP_VRTouch.IBP_VRTouching` (`self.GetAttachParentActor`) (`self.BID`) self "touchDamage")
  (`GameplayStatics.SpawnEmitterAtLocation` "/Game/GBL_Xreality/Fx/pa_TouchImpact.pa_TouchImpact" (`self.K2_GetActorLocation`)))

(event `self.ReceiveBeginPlay`
  (`parent.ReceiveBeginPlay`)
  (add `self.DOnTouch` (delegate `OnTouch`)))

(fn `UserConstructionScript`
  (`parent.UserConstructionScript`))