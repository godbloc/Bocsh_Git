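; House object for the BoschVR game with an adjustable dirt state, a clean/dirty effect and physics that can be switched on.
; The construction script creates a dynamic material and picks the StateFx template from CleanState.
; An interface event clamps a new alpha into the material's "state" parameter, with zero counting as clean.
; Runtime changes leave the effect template untouched, and the CleanState OnRep does nothing.
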(event `StartPhysic`
  (`PrimitiveComponent.SetSimulatePhysics` (`self.StaticMesh`) true))

(event `/Game/GBL_Xreality/Bp/Interfaces/IBP_XVR.Ibp_VRChangeStateAlpha`
  (params (NewState :type "Float (double-precision)") (Sender :type "Actor Object Reference") (Params :type String) (BID :type Integer))
  (bind _output_get (set `self.CurrentState` (`KismetMathLibrary.FClamp` NewState)))
  (`self.ApplyNewState` _output_get))

(event `ApplyNewState`
  (params (dirtAlpha :type "Float (single-precision)"))
  (`MaterialInstanceDynamic.SetScalarParameterValue` (`self.DynMap`) "state" dirtAlpha)
  (set `self.CleanState` (== dirtAlpha 0.0)))

(event `self.ReceiveBeginPlay`)

(fn `OnRep_CleanState`
  (if (`self.CleanState`)
    _))

(fn `UserConstructionScript`
  (bind _staticmesh (`self.StaticMesh`))
  (bind _statefx (`self.StateFx`))
  (`parent.UserConstructionScript`)
  (bind _returnvalue (`KismetMaterialLibrary.CreateDynamicMaterialInstance` (`PrimitiveComponent.GetMaterial` _staticmesh 0)))
  (bind _output_get (set `self.DynMap` _returnvalue))
  (`PrimitiveComponent.SetMaterial` _staticmesh 0 _output_get)
  (`self.ApplyNewState` (`self.CurrentState`))
  (if (`self.CleanState`)
    (`ParticleSystemComponent.SetTemplate` _statefx (`self.TrueFx`))
    (else
      (`ParticleSystemComponent.SetTemplate` _statefx (`self.falseFx`)))))